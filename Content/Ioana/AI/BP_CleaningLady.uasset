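; Cleaning lady AI character that spots and chases a target through AI perception, with visual alert feedback.
; Perception updates write the sensed actor to the Blackboard "Player" key and fire OnPlayerSpotted; forgetting clears the key and fires OnPlayerLost.
; When spotted, it freezes for a second under an exclamation mark, then walks at chase speed.
; A dynamic material on the detection radius turns red while chasing and green when the target is forgotten.
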(event OnTargetPerceptionUpdated(AIPerception)
  (params (Actor :type Actor%20Object%20Reference) (Stimulus :type AI%20Stimulus%20Structure))
  (if (not (Variables|Default|GetIsChasing))
    (AI|Components|Blackboard|SetValueasObject (AI|GetBlackboard (Pawn|GetController)) (Utilities|Name|MakeLiteralName "Player") Actor)
    (Default|CallOnPlayerSpotted)))

(event OnTargetPerceptionForgotten(AIPerception)
  (params (Actor :type Actor%20Object%20Reference))
  (AI|Components|Blackboard|ClearValue (AI|GetBlackboard (Pawn|GetController)) (Utilities|Name|MakeLiteralName "Player"))
  (Rendering|Material|SetVectorParameterValue (Variables|Default|GetDetectionRadiusMat) "Color" "(R=0.091608,G=1.000000,B=0.000000,A=1.000000)" :!class /Script/Engine.MaterialInstanceDynamic)
  (Variables|Default|SetIsChasing false)
  (Default|CallOnPlayerLost))

(event Custom|OnPlayerSpotted_Event
  (bind _charactermovement (Variables|Character|GetCharacterMovement))
  (bind _exclamation (Variables|Default|GetExclamation))
  (Variables|Default|SetIsChasing true)
  (Pawn|Components|CharacterMovement|DisableMovement (Variables|Character|GetCharacterMovement))
  (Rendering|SetVisibility _exclamation true false)
  (Rendering|Material|SetVectorParameterValue (Variables|Default|GetDetectionRadiusMat) "Color" "(R=1.000000,G=0.000000,B=0.009999,A=1.000000)" :!class /Script/Engine.MaterialInstanceDynamic)
  (Utilities|FlowControl|Delay 1.0)
  (Rendering|SetVisibility _exclamation false false)
  (Pawn|Components|CharacterMovement|SetMovementMode _charactermovement "MOVE_Walking" 0)
  (Variables|/Script/Engine.CharacterMovementComponent|SetMaxWalkSpeed _charactermovement 3e+02))

(event EventBeginPlay
  (EventDispatchers|BindEventtoOnPlayerSpotted (delegate Custom|OnPlayerSpotted_Event)))

(fn ConstructionScript
  (bind _returnvalue (Rendering|Material|CreateDynamicMaterialInstance (Variables|Default|GetDetectionRadius) 0 0 "None" :!class /Script/Engine.PrimitiveComponent))
  (Variables|Default|SetDetectionRadiusMat _returnvalue))