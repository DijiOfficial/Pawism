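; BP_Roomba is a Roomba actor that the player can mount and dismount through a toggling Mount event.
; Mounting teleports the player above the Roomba and attaches the Roomba to the player, so the player carries it along.
; Dismounting nudges the player forward along its local X axis and detaches the Roomba.
; Each branch flips IsMounted and fires the matching OnMounted or OnDismounted dispatcher.
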(event EventMount
  (params (Player :type Actor%20Object%20Reference))
  (if (Variables|Default|GetIsMounted)
    (Transformation|AddActorLocalOffset Player "100.000000,0.000000,0.000000" false false)
    (Transformation|DetachFromActor "KeepWorld" "KeepWorld" "KeepWorld")
    (Default|CallOnDismounted)
    (Variables|Default|SetIsMounted false)
    (else
      (Transformation|SetActorLocation Player (+ (Transformation|GetWorldLocation (Variables|Default|GetRoomba)) "0.000000,0.000000,100.000000") false false)
      (Transformation|AttachActorToActor Player "None" "KeepWorld" "KeepWorld" "KeepWorld" true)
      (Default|CallOnMounted)
      (Variables|Default|SetIsMounted true))))

(fn ConstructionScript)