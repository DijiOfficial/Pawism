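; Cleaning lady AI character that spots and chases the player's cat, BP_CatCharacter.
; AI perception writes or clears the Player blackboard key and fires spotted and lost events.
; Spotting turns the detection radius red, briefly freezes her with an exclamation mark and gasp, then starts chase music and sets chase walk speed.
; Forgetting the cat restores the green radius and swaps chase music for a funny soundtrack, using sound mixes.
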(event OnTargetPerceptionUpdated(AIPerception)
  (params (Actor :type Actor%20Object%20Reference) (Stimulus :type AI%20Stimulus%20Structure))
  (Utilities|Casting|CastToBP_CatCharacter Actor)
  (if (not (Variables|Default|GetIsChasing))
    (AI|Components|Blackboard|SetValueasObject (AI|GetBlackboard (Pawn|GetController)) (Utilities|Name|MakeLiteralName "Player") Actor)
    (Default|CallOnPlayerSpotted)))

(event OnTargetPerceptionForgotten(AIPerception)
  (params (Actor :type Actor%20Object%20Reference))
  (Utilities|Casting|CastToBP_CatCharacter Actor)
  (AI|Components|Blackboard|ClearValue (AI|GetBlackboard (Pawn|GetController)) (Utilities|Name|MakeLiteralName "Player"))
  (Rendering|Material|SetVectorParameterValue (Variables|Default|GetDetectionRadiusMat) "Color" "(R=0.091608,G=1.000000,B=0.000000,A=1.000000)" :!class /Script/Engine.MaterialInstanceDynamic)
  (Variables|Default|SetIsChasing false)
  (Default|CallOnPlayerLost)
  (Audio|Components|Audio|FadeOut (Variables|Default|GetChaseMusic) 0.0 0.0 "Linear" :!class /Script/Engine.AudioComponent)
  (Audio|PushSoundMixModifier "/Game/PlayMix.PlayMix")
  (Audio|PlaySound2D "/Game/igor/Sounds/Ambiences/FunnySoundtrack_Cue.FunnySoundtrack_Cue" 1.0 1.0 0.0 0 0))

(event Custom|OnPlayerSpotted_Event
  (bind _charactermovement (Variables|Character|GetCharacterMovement))
  (bind _exclamation (Variables|Default|GetExclamation))
  (Variables|Default|SetIsChasing true)
  (Pawn|Components|CharacterMovement|DisableMovement (Variables|Character|GetCharacterMovement))
  (Rendering|SetVisibility _exclamation true false)
  (Rendering|Material|SetVectorParameterValue (Variables|Default|GetDetectionRadiusMat) "Color" "(R=1.000000,G=0.000000,B=0.009999,A=1.000000)" :!class /Script/Engine.MaterialInstanceDynamic)
  (Audio|PushSoundMixModifier "/Game/igor/Sounds/SoundMixes/StopMixx.StopMixx")
  (Audio|PlaySoundatLocation "/Game/igor/Sounds/Metasounds/MSSource/MS_Gasp.MS_Gasp" (Transformation|GetActorLocation) "0, 0, 0" 1.0 1.0 0.0 0 0 0 0)
  (Utilities|FlowControl|Delay 0.8)
  (Audio|PopSoundMixModifier "/Game/igor/Sounds/SoundMixes/StopMixx.StopMixx")
  (Audio|Components|Audio|Play (Variables|Default|GetChaseMusic) 0.0)
  (Utilities|FlowControl|Delay 1.0)
  (Rendering|SetVisibility _exclamation false false)
  (Pawn|Components|CharacterMovement|SetMovementMode _charactermovement "MOVE_Walking" 0)
  (Variables|/Script/Engine.CharacterMovementComponent|SetMaxWalkSpeed _charactermovement 3e+02))

(event EventBeginPlay
  (EventDispatchers|BindEventtoOnPlayerSpotted (delegate Custom|OnPlayerSpotted_Event)))

(event EventTick
  (params (DeltaSeconds :type Float%20%28single-precision%29)))

(fn ConstructionScript
  (bind _returnvalue (Rendering|Material|CreateDynamicMaterialInstance (Variables|Default|GetDetectionRadius) 0 0 "None" :!class /Script/Engine.PrimitiveComponent))
  (Variables|Default|SetDetectionRadiusMat _returnvalue))