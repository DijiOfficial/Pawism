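; BP_GameModeMinigame is the game mode for a minigame, handling the player being caught and the start of play.
; When the player is caught it shows the W_GotCaught widget, pauses the game, and opens the L_AiDebug level once that widget's animation finishes.
; StartGame unpauses and clears all widgets.
; Logic to show a paused W_StartMenu with a focused start button is disconnected and never runs.
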(event Custom|OnPlayerCaught
  (bind _returnvalue (UserInterface|CreateWidget "/Game/Paw_ism/Core/Widgets/W_GotCaught.W_GotCaught_C"))
  (UserInterface|Viewport|AddtoViewport _returnvalue 0)
  (Game|SetGamePaused true)
  (EventDispatchers|AssignOnAnimFinished _returnvalue (delegate Custom|OnAnimFinished_Event)))

(event Custom|OnAnimFinished_Event
  (Game|OpenLevel(byObjectReference) "/Game/Ioana/L_AiDebug.L_AiDebug"))

(event Custom|StartGame
  (Game|SetGamePaused false)
  (Viewport|RemoveAllWidgets))

(event EventBeginPlay)

(event EventTick
  (params (DeltaSeconds :type Float%20%28single-precision%29)))

(fn ConstructionScript)