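; BP_Paw is a minigame paw actor that continuously turns to track the player.
; It caches the first player's pawn on BeginPlay.
; Each Tick it sets the PawPivot component's world rotation from the direction to that pawn, using MakeRotFromY so the pivot's Y axis, rather than X, points at the player.
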(event EventBeginPlay
  (Variables|Default|SetPlayer (Game|Player|GetPlayerPawn 0)))

(event Collision|EventActorBeginOverlap
  (params (OtherActor :type Actor%20Object%20Reference)))

(event EventTick
  (params (DeltaSeconds :type Float%20%28single-precision%29))
  (bind _player (Variables|Default|GetPlayer))
  (bind _pawpivot (Variables|Default|GetPawPivot))
  (bind _returnvalue (Transformation|GetActorLocation _player))
  (bind _returnvalue_2 (Transformation|GetWorldLocation _pawpivot))
  (bind _returnvalue_3 (- _returnvalue _returnvalue_2))
  (bind _returnvalue_4 (Math|Rotator|MakeRotfromY _returnvalue_3))
  (Transformation|SetWorldRotation _pawpivot (Math|Rotator|MakeRotator (.roll _returnvalue_4) (.pitch _returnvalue_4) (.yaw _returnvalue_4)) false false))

(fn ConstructionScript)