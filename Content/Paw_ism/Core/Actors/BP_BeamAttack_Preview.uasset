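; BP_BeamAttack_Preview is a short-lived actor that, by its name, previews a beam attack.
; On BeginPlay it reads the forward vector of the BP_GOD actor in the level and teleports its Box component a fixed distance along that direction, without sweeping.
; The offset applies immediately, while a parallel sequence branch destroys the actor after a one-second delay.
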(event EventBeginPlay
  (Utilities|FlowControl|Sequence
    (:then_0
      (bind _returnvalue (Actor|GetActorOfClass "/Game/Paw_ism/Core/Characters/BP_GOD.BP_GOD_C"))
      (Variables|Default|SetDirection (Transformation|GetActorForwardVector _returnvalue)))
    (:then_1
      (Utilities|FlowControl|Delay 1.0)
      (Actor|DestroyActor))
    (:then_2
      (Transformation|AddWorldOffset (Variables|Default|GetBox) (* (Variables|Default|GetDirection) (Math|Float|MakeLiteralFloat 4e+02)) false true))))

(event EventTick
  (params (DeltaSeconds :type Float%20%28single-precision%29)))

(fn ConstructionScript)