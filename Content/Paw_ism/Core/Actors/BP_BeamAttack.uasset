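; BP_BeamAttack is a short-lived beam attack actor that damages the player's cat character.
; On BeginPlay it takes the forward vector of the BP_GOD actor, immediately teleports its Box collision along that direction and destroys itself after a short delay.
; While CanDamage is set, a cat overlapping the Box gets DoDamageMessage on its BP_Health_AC component, then the flag clears to limit the beam to one hit.
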(event OnComponentBeginOverlap(Box)
  (params (OverlappedComponent :type Primitive%20Component%20Object%20Reference) (OtherActor :type Actor%20Object%20Reference) (OtherComp :type Primitive%20Component%20Object%20Reference) (OtherBodyIndex :type Integer) (bFromSweep :type Boolean) (SweepResult :type Hit%20Result%20Structure%20%28by%20ref%29))
  (if (Variables|Default|GetCanDamage)
    (bind _asbp_cat_character (Utilities|Casting|CastToBP_CatCharacter OtherActor))
    (Class|BPIDamageable|DoDamage(Message) (Actor|GetComponentbyClass _asbp_cat_character "/Game/dylan/BP_Health_AC.BP_Health_AC_C"))
    (Variables|Default|SetCanDamage false)))

(event EventBeginPlay
  (Utilities|FlowControl|Sequence
    (:then_0
      (bind _returnvalue (Actor|GetActorOfClass "/Game/Paw_ism/Core/Characters/BP_GOD.BP_GOD_C"))
      (Variables|Default|SetDirection (Transformation|GetActorForwardVector _returnvalue)))
    (:then_1
      (Utilities|FlowControl|Delay 3.0)
      (Actor|DestroyActor))
    (:then_2
      (Transformation|AddWorldOffset (Variables|Default|GetBox) (* (Variables|Default|GetDirection) (Math|Float|MakeLiteralFloat 4e+02)) false true))))

(event EventTick
  (params (DeltaSeconds :type Float%20%28single-precision%29)))

(fn ConstructionScript)