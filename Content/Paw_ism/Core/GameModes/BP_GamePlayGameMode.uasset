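; Game mode for the gameplay level that manages the start menu, the switch into play and the restart when the player is caught.
; BeginPlay shows the start menu, then focuses its start button and pauses the game after a short delay.
; StartGame unpauses and swaps the menu for the HUD and task widgets.
; OnPlayerCaught resets the game instance, pauses behind a caught screen and reloads L_GamePlay when its animation finishes.
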(event Custom|OnPlayerCaught
  (Default|FullReset (.AsBP%20My%20Game%20Instanc (Utilities|Casting|CastToBP_MyGameInstanc (Game|GetGameInstance))))
  (bind _returnvalue (UserInterface|CreateWidget "/Game/Paw_ism/Core/Widgets/W_GotCaught.W_GotCaught_C"))
  (UserInterface|Viewport|AddtoViewport _returnvalue 0)
  (Game|SetGamePaused true)
  (EventDispatchers|AssignOnAnimFinished _returnvalue (delegate Custom|OnAnimFinished_Event)))

(event Custom|OnAnimFinished_Event
  (Game|OpenLevel(byObjectReference) "/Game/Paw_ism/Maps/L_GamePlay.L_GamePlay"))

(event Custom|StartGame
  (Game|SetGamePaused false)
  (Widget|RemovefromParent (Variables|Default|GetStartMenu))
  (bind _returnvalue (UserInterface|CreateWidget "/Game/dylan/W_HUD.W_HUD_C"))
  (UserInterface|Viewport|AddtoViewport _returnvalue 0)
  (bind _returnvalue_2 (UserInterface|CreateWidget "/Game/Paw_ism/Core/Widgets/W_Tasks.W_Tasks_C"))
  (UserInterface|Viewport|AddtoViewport _returnvalue_2 0))

(event EventBeginPlay
  (bind _returnvalue (UserInterface|CreateWidget "/Game/Paw_ism/Core/Widgets/W_StartMenu.W_StartMenu_C"))
  (Variables|Default|SetStartMenu _returnvalue)
  (UserInterface|Viewport|AddtoViewport _returnvalue 0)
  (Input|SetInputModeGameandUI (Game|GetPlayerController 0) _returnvalue "DoNotLock" true false)
  (Utilities|FlowControl|Delay 0.5)
  (Widget|SetKeyboardFocus (Variables|/Game/Paw_ism/Core/Widgets/W_StartMenu.W_StartMenu_C|GetStartButton _returnvalue))
  (Game|SetGamePaused true))

(fn ConstructionScript)