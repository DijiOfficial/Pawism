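; BP_CatController is the cat player's controller, switching possession between the cat pawn and a minigame character.
; On BeginPlay it sets the view to the gameplay camera, caches both pawns, and binds to every mouse hole and, a tick later, the start menu.
; A mouse hole interaction possesses the minigame pawn.
; Game start hooks the HUD's minigame timer, whose end returns possession to the cat.
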(event Custom|MouseHoleInteracted_Event
  (Pawn|Possess (Variables|Default|GetMinigamePawn)))

(event Custom|OnMinigameTimerEnd_Event
  (Pawn|Possess (Variables|Default|GetCatPawn))
  (Development|PrintString " possessed cat"))

(event Custom|OnGameStartEvent_Event
  (bind _foundwidgets (Widget|GetAllWidgetsOfClass "/Game/dylan/W_HUD.W_HUD_C" true))
  (EventDispatchers|AssignOnMinigameTimerEnd (Utilities|Array|Get(acopy) _foundwidgets) (delegate Custom|OnMinigameTimerEnd_Event)))

(event EventBeginPlay
  (Utilities|FlowControl|Sequence
    (:then_0
      (bind _returnvalue (Actor|GetActorOfClass "/Game/Paw_ism/Core/Camera/BP_GamePlayCamera.BP_GamePlayCamera_C"))
      (Game|Player|SetViewTargetwithBlend _returnvalue 0.0 "VTBlend_Linear" 0.0 false)
      (bind _outactors (Actor|GetAllActorsOfClass "/Game/Ioana/Minigame/BP_MinigameChar.BP_MinigameChar_C"))
      (Variables|Default|SetMinigamePawn (Utilities|Array|Get(acopy) _outactors))
      (Utilities|FlowControl|Sequence
        (:then_0
          (bind _outactors_2 (Actor|GetAllActorsOfClass "/Game/dylan/BP_MouseHole.BP_MouseHole_C"))
          (for _array_element _outactors_2
            (EventDispatchers|AssignMouseHoleInteracted _array_element (delegate Custom|MouseHoleInteracted_Event))))
        (:then_1
          (Utilities|FlowControl|DelayUntilNextTick)
          (bind _foundwidgets (Widget|GetAllWidgetsOfClass "/Game/Paw_ism/Core/Widgets/W_StartMenu.W_StartMenu_C" true))
          (for _array_element_2 _foundwidgets
            (EventDispatchers|AssignOnGameStartEvent _array_element_2 (delegate Custom|OnGameStartEvent_Event))))))
    (:then_1
      (Utilities|FlowControl|DelayUntilNextTick)
      (Variables|Default|SetCatPawn (Game|Player|GetPlayerPawn 0)))))

(fn ConstructionScript)