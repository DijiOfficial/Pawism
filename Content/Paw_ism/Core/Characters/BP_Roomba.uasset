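; BP_Roomba is a Roomba that the player can mount and dismount, and that draws AI attention while ridden.
; Mount toggles state: it moves the player to the Center socket and attaches the Roomba to the player, or detaches it.
; Each toggle calls the matching mounted or dismounted notification.
; The Roomba's sound starts on BeginPlay, and Tick reports a noise event at its mesh every frame while mounted.
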(event EventMount
  (params (Player :type Actor%20Object%20Reference))
  (if (Variables|Default|GetIsMounted)
    ;[0.15 0.15 0.15 0.5] Mount
    (Transformation|DetachFromActor "KeepWorld" "KeepWorld" "KeepWorld")
    (Default|CallOnDismounted)
    (Variables|Default|SetIsMounted false)
    (else
      ;[0.15 0.15 0.15 0.5] Dismount
      (Transformation|SetActorLocation Player (Transformation|GetSocketLocation (Variables|Default|Getroomba_Final) "Center") false false)
      (Transformation|AttachActorToActor Player "None" "KeepWorld" "KeepWorld" "KeepWorld" true)
      (Default|CallOnMounted)
      (Variables|Default|SetIsMounted true))))

(event EventBeginPlay
  ;[0.15 0.15 0.15 0.5] Play sound
  (Audio|Components|Audio|Play (Variables|Default|GetRoombaSound) 0.0))

(event EventTick
  (params (DeltaSeconds :type Float%20%28single-precision%29))
  ;[0.15 0.15 0.15 0.5] Make noise while mounted
  (if (Variables|Default|GetIsMounted)
    (Class|AISenseHearing|ReportNoiseEvent (Transformation|GetWorldLocation (Variables|Character|GetMesh)) 1.0 self 0.0 "None")))

(fn ConstructionScript)