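; BP_RoomTrigger manages a room's camera move, lighting and ambient audio.
; TransitionCameraEvent slides BP_GamePlayCamera to a target point with a timeline lerp, toggles the room's lights, plays its ambient sound and attaches the audio listener to ListenerLocation.
; Separate custom events stop the transition or toggle lights and silence audio, replacing the now-inert cat overlap handlers.
; An optional flag toggles the lights on BeginPlay.
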(event Custom|TransitionCamera
  (bind _time (Timeline|Transition PlayFromStart)
    (:Update
      (Transformation|SetActorLocation (Variables|Default|GetCamera) (Math|Vector|Lerp(Vector) (Variables|Default|GetInitialPosition) (Transformation|GetActorLocation (Variables|Default|GetTargetPoint)) _time) false false))))

(event Custom|TransitionCameraEvent
  (bind _listenerlocation (Variables|Default|GetListenerLocation))
  (bind _audio (Variables|Default|GetAudio))
  ;[0 0 0 0.5] Camera original position
  (Variables|Default|SetInitialPosition (Transformation|GetActorLocation (Variables|Default|GetCamera)))
  (CallFunction|TransitionCamera)
  (CallFunction|ToggleLights)
  (Audio|Components|Audio|SetSound _audio (Variables|Default|GetAmbientZone))
  (Audio|Components|Audio|Play _audio 0.0)
  (Class|PlayerController|SetAudioListenerOverride (Game|GetPlayerController 0) _listenerlocation (Transformation|GetWorldLocation _listenerlocation) "0, 0, 0"))

(event Custom|ToggleLightsEvent
  (CallFunction|ToggleLights)
  (Audio|Components|Audio|Stop (Variables|Default|GetAudio)))

(event Custom|StopTransitionCameraEvent
  (bind _time (Timeline|Transition Stop)
    (:Update
      (Transformation|SetActorLocation (Variables|Default|GetCamera) (Math|Vector|Lerp(Vector) (Variables|Default|GetInitialPosition) (Transformation|GetActorLocation (Variables|Default|GetTargetPoint)) _time) false false))))

(event EventBeginPlay
  ;[0 0 0 0.5] Get Camera reference
  (bind _returnvalue (Actor|GetActorOfClass "/Game/Paw_ism/Core/Camera/BP_GamePlayCamera.BP_GamePlayCamera_C"))
  (Variables|Default|SetCamera _returnvalue)
  ;[0 0 0 0.5] Toggle Light
  (if (Variables|Default|GetbToggleLight)
    (CallFunction|ToggleLights)))

(event Collision|EventActorBeginOverlap
  (params (OtherActor :type Actor%20Object%20Reference))
  ;[0.15 0.15 0.15 0.5] Unused at the moment - replaced by custom events
  (Utilities|Casting|CastToBP_CatCharacter OtherActor))

(event Collision|EventActorEndOverlap
  (params (OtherActor :type Actor%20Object%20Reference))
  ;[0.15 0.15 0.15 0.5] Unused at the moment - replaced by custom events
  (Utilities|Casting|CastToBP_CatCharacter OtherActor))

(fn ConstructionScript)

(fn ToggleLights
  (for _array_element (Variables|Default|GetLights)
    (Rendering|ToggleVisibility (Variables|/Script/Engine.Actor|GetRootComponent _array_element) false)))