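; Ritual triangle actor that the cat completes with dead mice and a Roomba, notifying the game instance through PentagramDrawn.
; MouseTrigger spends carried mice from the game instance to fill up to three corners.
; Overlapping a filled corner while on the Roomba activates it once, swapping the mouse for blood effects, sound and a fading-in line.
; Tick polls for all three corners to fire completion and smoke, while timelines grow and reverse blood-pool decals.
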(event OnComponentBeginOverlap(Corner3Trigger)
  (params (OverlappedComponent :type Primitive%20Component%20Object%20Reference) (OtherActor :type Actor%20Object%20Reference) (OtherComp :type Primitive%20Component%20Object%20Reference) (OtherBodyIndex :type Integer) (bFromSweep :type Boolean) (SweepResult :type Hit%20Result%20Structure%20%28by%20ref%29))
  ;[0 0 0 0.5] Has enough mice && is on roomba?
  (bind _asbp_cat_character (Utilities|Casting|CastToBP_CatCharacter OtherActor))
  (if (and (Variables|/Game/Paw_ism/Core/Characters/BP_CatCharacter.BP_CatCharacter_C|GetbOnRoomba _asbp_cat_character) (Variables|Default|GetbThirdMouse))
    (Utilities|FlowControl|DoOnce false
      (:Completed
        (Variables|Default|SetbThirdActive true)
        ;[0.15 0.15 0.15 0.5] Hide mouse
        (Rendering|ToggleVisibility (Variables|Default|GetMouse3) false)
        (Rendering|ToggleVisibility (Variables|Default|GetLine3) false)
        ;[0.15 0.15 0.15 0.5] blood pool
        (CallFunction|SpawnBloodPool (Transformation|GetWorldLocation (Variables|Default|GetBloodSpot3)))
        ;[0.15 0.15 0.15 0.5] Fade in blood
        (bind _returnvalue (Rendering|Material|CreateDynamicMaterialInstance "/Game/adam/M_FadeIn.M_FadeIn" "None" "None" :!class /Script/Engine.KismetMaterialLibrary))
        (Rendering|Material|SetMaterial (Variables|Default|GetLine3) 0 _returnvalue)
        (bind _time (Timeline|Timeline_2 Play)
          (:Update
            (Rendering|Material|SetScalarParameterValue _returnvalue "FadeAmount" _time :!class /Script/Engine.MaterialInstanceDynamic)
            ;[0.15 0.15 0.15 0.5] Mouse Flesh
            (Utilities|FlowControl|DoOnce false
              (:Completed
                (Niagara|SpawnSystematLocation "/Game/adam/NS_Blood.NS_Blood" (Transformation|GetWorldLocation (Variables|Default|GetBloodSpot3)))
                ;[0.15 0.15 0.15 0.5] Sound
                (Audio|PlaySound2D "/Game/igor/Sounds/Metasounds/MSSource/MS_Blood.MS_Blood" 1.0 1.0 0.0 0 0)
                (Audio|PlaySound2D "/Game/igor/Sounds/Source/Boom/boomer.boomer" 1.0 1.0 0.0 0 0)))))))))

(event OnComponentBeginOverlap(Corner2Trigger)
  (params (OverlappedComponent :type Primitive%20Component%20Object%20Reference) (OtherActor :type Actor%20Object%20Reference) (OtherComp :type Primitive%20Component%20Object%20Reference) (OtherBodyIndex :type Integer) (bFromSweep :type Boolean) (SweepResult :type Hit%20Result%20Structure%20%28by%20ref%29))
  ;[0 0 0 0.5] Has enough mice && is on roomba?
  (bind _asbp_cat_character (Utilities|Casting|CastToBP_CatCharacter OtherActor))
  (if (and (Variables|/Game/Paw_ism/Core/Characters/BP_CatCharacter.BP_CatCharacter_C|GetbOnRoomba _asbp_cat_character) (Variables|Default|GetbSecondMouse))
    (Utilities|FlowControl|DoOnce false
      (:Completed
        (Variables|Default|SetbSecondActive true)
        ;[0.15 0.15 0.15 0.5] Hide mouse
        (Rendering|ToggleVisibility (Variables|Default|GetMouse2) false)
        (Rendering|ToggleVisibility (Variables|Default|GetLine2) false)
        ;[0.15 0.15 0.15 0.5] blood pool
        (CallFunction|SpawnBloodPool (Transformation|GetWorldLocation (Variables|Default|GetBloodSpot2)))
        ;[0.15 0.15 0.15 0.5] Fade in blood
        (bind _returnvalue (Rendering|Material|CreateDynamicMaterialInstance "/Game/adam/M_FadeIn.M_FadeIn" "None" "None" :!class /Script/Engine.KismetMaterialLibrary))
        (Rendering|Material|SetMaterial (Variables|Default|GetLine2) 0 _returnvalue)
        (bind _time (Timeline|Timeline_1 Play)
          (:Update
            (Rendering|Material|SetScalarParameterValue _returnvalue "FadeAmount" _time :!class /Script/Engine.MaterialInstanceDynamic)
            ;[0.15 0.15 0.15 0.5] Mouse Flesh
            (Utilities|FlowControl|DoOnce false
              (:Completed
                (Niagara|SpawnSystematLocation "/Game/adam/NS_Blood.NS_Blood" (Transformation|GetWorldLocation (Variables|Default|GetBloodSpot2)))
                ;[0.15 0.15 0.15 0.5] Sound
                (Audio|PlaySound2D "/Game/igor/Sounds/Metasounds/MSSource/MS_Blood.MS_Blood" 1.0 1.0 0.0 0 0)
                (Audio|PlaySound2D "/Game/igor/Sounds/Source/Boom/boomer.boomer" 1.0 1.0 0.0 0 0)))))))))

(event OnComponentBeginOverlap(Corner1Trigger)
  (params (OverlappedComponent :type Primitive%20Component%20Object%20Reference) (OtherActor :type Actor%20Object%20Reference) (OtherComp :type Primitive%20Component%20Object%20Reference) (OtherBodyIndex :type Integer) (bFromSweep :type Boolean) (SweepResult :type Hit%20Result%20Structure%20%28by%20ref%29))
  ;[0 0 0 0.5] Has enough mice && is on roomba?
  (bind _asbp_cat_character (Utilities|Casting|CastToBP_CatCharacter OtherActor))
  (if (and (Variables|/Game/Paw_ism/Core/Characters/BP_CatCharacter.BP_CatCharacter_C|GetbOnRoomba _asbp_cat_character) (Variables|Default|GetbFirstMouse))
    (Utilities|FlowControl|DoOnce false
      (:Completed
        (Variables|Default|SetbFirstActive true)
        ;[0.15 0.15 0.15 0.5] Hide mouse
        (Rendering|ToggleVisibility (Variables|Default|GetMouse1) false)
        (Rendering|ToggleVisibility (Variables|Default|GetLine1) false)
        ;[0.15 0.15 0.15 0.5] blood pool
        (CallFunction|SpawnBloodPool (Transformation|GetWorldLocation (Variables|Default|GetBloodSpot1)))
        ;[0.15 0.15 0.15 0.5] Fade in blood
        (bind _returnvalue (Rendering|Material|CreateDynamicMaterialInstance "/Game/adam/M_FadeIn.M_FadeIn" "None" "None" :!class /Script/Engine.KismetMaterialLibrary))
        (Rendering|Material|SetMaterial (Variables|Default|GetLine1) 0 _returnvalue)
        (bind _time (Timeline|Timeline_0 Play)
          (:Update
            (Rendering|Material|SetScalarParameterValue _returnvalue "FadeAmount" _time :!class /Script/Engine.MaterialInstanceDynamic)
            ;[0.15 0.15 0.15 0.5] Mouse Flesh
            (Utilities|FlowControl|DoOnce false
              (:Completed
                (Niagara|SpawnSystematLocation "/Game/adam/NS_Blood.NS_Blood" (Transformation|GetWorldLocation (Variables|Default|GetBloodSpot1)))
                ;[0.15 0.15 0.15 0.5] Sound
                (Audio|PlaySound2D "/Game/igor/Sounds/Metasounds/MSSource/MS_Blood.MS_Blood" 1.0 1.0 0.0 0 0)
                (Audio|PlaySound2D "/Game/igor/Sounds/Source/Boom/boomer.boomer" 1.0 1.0 0.0 0 0)))))))))

(event OnComponentBeginOverlap(MouseTrigger)
  (params (OverlappedComponent :type Primitive%20Component%20Object%20Reference) (OtherActor :type Actor%20Object%20Reference) (OtherComp :type Primitive%20Component%20Object%20Reference) (OtherBodyIndex :type Integer) (bFromSweep :type Boolean) (SweepResult :type Hit%20Result%20Structure%20%28by%20ref%29))
  ;[0.15 0.15 0.15 0.5] Has enough mice?
  (Utilities|Casting|CastToBP_CatCharacter OtherActor)
  (bind _asbp_my_game_instanc (Utilities|Casting|CastToBP_MyGameInstanc (Game|GetGameInstance)))
  (bind _newparam (Default|HasMouse _asbp_my_game_instanc))
  (if (and _newparam (not (Variables|Default|GetbFirstMouse)))
    ;[0.15 0.15 0.15 0.5] Show 1 dead mouse
    (Rendering|ToggleVisibility (Variables|Default|GetMouse1) false)
    (Variables|Default|SetbFirstMouse true)
    (Default|DecrementMice _asbp_my_game_instanc))
  (bind _newparam_2 (Default|HasMouse _asbp_my_game_instanc))
  (if (and _newparam_2 (not (Variables|Default|GetbSecondMouse)))
    ;[0.15 0.15 0.15 0.5] Show 2 dead mice
    (Rendering|ToggleVisibility (Variables|Default|GetMouse2) false)
    (Variables|Default|SetbSecondMouse true)
    (Default|DecrementMice _asbp_my_game_instanc))
  (bind _newparam_3 (Default|HasMouse _asbp_my_game_instanc))
  (if (and _newparam_3 (not (Variables|Default|GetbThirdMouse)))
    ;[0.15 0.15 0.15 0.5] Show 3 dead mice
    (Rendering|ToggleVisibility (Variables|Default|GetMouse3) false)
    (Variables|Default|SetbThirdMouse true)
    (Default|DecrementMice _asbp_my_game_instanc)))

(event Custom|SoakUpBlood
  (params (BloodPool :type Material%20Instance%20Dynamic%20Object%20Reference))
  ;[0.15 0.15 0.15 0.5] Reverse blood spot effect
  (bind _newtrack_0 (Timeline|Reverse PlayFromStart)
    (:Update
      (Rendering|Material|SetScalarParameterValue BloodPool "Time" (Math|Float|Clamp(Float) _newtrack_0 0.0 0.999) :!class /Script/Engine.MaterialInstanceDynamic))))

(event Custom|SpawnBloodPool
  (params (BloodPoolLocation :type Vector))
  (bind _returnvalue (Rendering|Material|CreateDynamicMaterialInstance "/Game/adam/MI_BloodPool.MI_BloodPool" "None" "None" :!class /Script/Engine.KismetMaterialLibrary))
  (Rendering|Decal|SpawnDecalatLocation _returnvalue (Variables|Default|GetDecalSize) BloodPoolLocation "-90.000000,0.000000,0.000000" 6e+01)
  (bind _alpha (Timeline|Timeline Play)
    (:Update
      (Rendering|Material|SetScalarParameterValue _returnvalue "Time" (Math|Float|Clamp(Float) _alpha 0.0 0.999) :!class /Script/Engine.MaterialInstanceDynamic))
    (:Finished
      (CallFunction|SoakUpBlood _returnvalue))))

(event EventTick
  (params (DeltaSeconds :type Float%20%28single-precision%29))
  ;[0.15 0.15 0.15 0.5] Triangle is complete
  (if (Math|Boolean|ANDBoolean (Variables|Default|GetbFirstActive) (Variables|Default|GetbSecondActive) (Variables|Default|GetbThirdActive))
    ;[0.15 0.15 0.15 0.5] Update game state
    (Utilities|FlowControl|DoOnce false
      (:Completed
        (Default|PentagramDrawn (.AsBP%20My%20Game%20Instanc (Utilities|Casting|CastToBP_MyGameInstanc (Game|GetGameInstance))))
        ;[0.15 0.15 0.15 0.5] Smoke effect
        (Niagara|SpawnSystematLocation "/Game/raluca/VFX/smoke_ns.smoke_ns" (Transformation|GetWorldLocation (Variables|Default|GetSmokeLocation)))))))

(fn ConstructionScript)