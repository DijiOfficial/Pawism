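; BP_RoomTrigger is a room trigger that moves the camera and toggles the room's lights when BP_Cat overlaps it.
; On enter, a Transition timeline lerps the BP_Camera found at BeginPlay from its current location to TargetPoint, moving position only.
; ToggleLights flips root component visibility on each actor in Lights on enter and exit, and at BeginPlay if ToggleLight is set.
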(event Custom|TransitionCamera
  (bind _time (Timeline|Transition PlayFromStart)
    (:Update
      (Transformation|SetActorLocation (Variables|Default|GetCamera) (Math|Vector|Lerp(Vector) (Variables|Default|GetInitialPosition) (Transformation|GetActorLocation (Variables|Default|GetTargetPoint)) _time) false false))))

(event EventBeginPlay
  ;[0 0 0 0.5] Get Camera reference
  (bind _returnvalue (Actor|GetActorOfClass "/Game/adam/BP_Camera.BP_Camera_C"))
  (Variables|Default|SetCamera _returnvalue)
  ;[0 0 0 0.5] Toggle Light
  (if (Variables|Default|GetbToggleLight)
    (CallFunction|ToggleLights)))

(event Collision|EventActorBeginOverlap
  (params (OtherActor :type Actor%20Object%20Reference))
  (Utilities|Casting|CastToBP_Cat OtherActor)
  ;[0 0 0 0.5] Camera original position
  (Variables|Default|SetInitialPosition (Transformation|GetActorLocation (Variables|Default|GetCamera)))
  (CallFunction|TransitionCamera)
  (CallFunction|ToggleLights))

(event Collision|EventActorEndOverlap
  (params (OtherActor :type Actor%20Object%20Reference))
  (Utilities|Casting|CastToBP_Cat OtherActor)
  (CallFunction|ToggleLights))

(fn ConstructionScript)

(fn ToggleLights
  (for _array_element (Variables|Default|GetLights)
    (Rendering|ToggleVisibility (Variables|/Script/Engine.Actor|GetRootComponent _array_element) false)))