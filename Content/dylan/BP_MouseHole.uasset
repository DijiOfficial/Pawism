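; Mouse hole interactable that takes the cat into a mouse-eating minigame.
; Overlap shows a camera-facing prompt; interacting runs a timed progress widget, then a Timeline moves the camera into the hole, teleports it to the target and spawns mice.
; The HUD timer ending, or a request to the HUD once this hole's mice or the overall quota are eaten, returns the camera and destroys leftover BP_Food.
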(event OnComponentBeginOverlap(Box)
  (params (OverlappedComponent :type Primitive%20Component%20Object%20Reference) (OtherActor :type Actor%20Object%20Reference) (OtherComp :type Primitive%20Component%20Object%20Reference) (OtherBodyIndex :type Integer) (bFromSweep :type Boolean) (SweepResult :type Hit%20Result%20Structure%20%28by%20ref%29))
  (bind _text (Variables|Default|Gettext))
  (Utilities|Casting|CastToBP_CatCharacter OtherActor)
  (if (not (Variables|/Script/Engine.SceneComponent|GetbVisible _text))
    (Rendering|SetVisibility _text true false)))

(event OnComponentEndOverlap(Box)
  (params (OverlappedComponent :type Primitive%20Component%20Object%20Reference) (OtherActor :type Actor%20Object%20Reference) (OtherComp :type Primitive%20Component%20Object%20Reference) (OtherBodyIndex :type Integer))
  (bind _eat_timer (Variables|Default|Geteat%20timer))
  (bind _text (Variables|Default|Gettext))
  (Utilities|Casting|CastToBP_CatCharacter OtherActor)
  (Utilities|FlowControl|Sequence
    (:then_0
      (if (Variables|Default|GetIsBeingEaten)
        (CallFunction|StopInteracting)
        (if (Variables|/Script/Engine.SceneComponent|GetbVisible _eat_timer)
          (Rendering|SetVisibility _eat_timer false false))))
    (:then_1
      (Utilities|FlowControl|DelayUntilNextTick)
      (if (Variables|/Script/Engine.SceneComponent|GetbVisible _text)
        (Rendering|SetVisibility _text false false)))))

(event Custom|OnMouseEatenEvent_Event
  (if (Variables|Default|GetIsActive)
    (bind _result (Math|Integer|DecrementInt (Variables|Default|GetMouseToSpawn))
      (:%20%20
        (if (or (== (Default|GetTotalMicePercent (.AsBP%20My%20Game%20Instanc (Utilities|Casting|CastToBP_MyGameInstanc (Game|GetGameInstance)))) 1.0) (== _result 0))
          (bind _foundwidgets (Widget|GetAllWidgetsOfClass "/Game/dylan/W_HUD.W_HUD_C" true))
          (Default|ReturnfromMiningame (Utilities|Array|Get(acopy) _foundwidgets)))))))

(event Custom|EatFood
  (bind _self self)
  (bind _eat_timer (Variables|Default|Geteat%20timer))
  (bind _camera (Variables|Default|GetCamera))
  (bind _camera_2 (Variables|Default|GetCamera))
  (bind _returnvalue (Transformation|GetActorLocation _self))
  (Development|PrintString "going to minigame")
  (Variables|Default|SetInitialPos (Transformation|GetWorldLocation (Variables|/Game/Paw_ism/Core/Camera/BP_GamePlayCamera.BP_GamePlayCamera_C|GetCamera _camera)))
  (Variables|Default|SetDefaultCamTransform (Transformation|GetWorldTransform (Variables|/Game/Paw_ism/Core/Camera/BP_GamePlayCamera.BP_GamePlayCamera_C|GetDefaultSceneRoot _camera)))
  (Default|CallMouseHoleInteracted)
  (if (Variables|/Script/Engine.SceneComponent|GetbVisible _eat_timer)
    (Rendering|SetVisibility _eat_timer false false)
    (bind _time (Timeline|Timeline PlayFromStart)
      (:Update
        (Transformation|SetActorLocation _camera_2 (Math|Vector|Lerp(Vector) (Variables|Default|GetInitialPos) (Math|Vector|MakeVector (.x _returnvalue) (.y _returnvalue) 0.0) _time) false false))
      (:Finished
        (Transformation|SetActorRotation _camera_2 "-65.000000,0.000000,0.000000")
        (Transformation|SetActorLocation _camera_2 (Transformation|GetActorLocation (Variables|Default|GetTarget)) false true)
        (if (> (Variables|Default|GetMouseToSpawn) 0)
          (for _index (range 1 (Variables|Default|GetMouseToSpawn))
            (Default|Spawn (Variables|Default|GetSpawner))))
        (Variables|Default|SetIsActive true)
        (Default|CallOnCameraTeleportedEvent)))
    (else
      (Timeline|Timeline PlayFromStart))))

(event Custom|OnMinigameTimerEnd_Event
  (bind _self self)
  (bind _defaultcamtransform (Variables|Default|GetDefaultCamTransform))
  (bind _camera (Variables|Default|GetCamera))
  (bind _text (Variables|Default|Gettext))
  (bind _returnvalue (Transformation|GetActorLocation _self))
  (bind _returnvalue_2 (Math|Vector|MakeVector (.x _returnvalue) (.y _returnvalue) 0.0))
  (if (Variables|Default|GetIsActive)
    (Variables|Default|SetIsActive false)
    (if (Variables|/Script/Engine.SceneComponent|GetbVisible _text)
      _
      (else
        (Rendering|SetVisibility _text true false)))
    (Utilities|FlowControl|Delay 0.85)
    (Transformation|SetActorLocation (Variables|Default|GetCamera) _returnvalue_2 false true)
    (Default|CallOnCameraTeleportBackEvent)
    (Transformation|SetActorRotation _camera (.rotation _defaultcamtransform))
    (bind _time (Timeline|Timeline_0 PlayFromStart)
      (:Update
        (Transformation|SetActorLocation _camera (Math|Vector|Lerp(Vector) _returnvalue_2 (.location _defaultcamtransform) _time) false false))
      (:Finished
        (bind _outactors (Actor|GetAllActorsOfClass "/Game/Ioana/BP_Food.BP_Food_C"))
        (for _array_element _outactors
          (Actor|DestroyActor _array_element)
          (Default|CallOnReturnfromMinigame))))))

(event Custom|ToggleEating
  (Variables|Default|SetCanEat (not (== (Default|GetTotalMicePercent (.AsBP%20My%20Game%20Instanc (Utilities|Casting|CastToBP_MyGameInstanc (Game|GetGameInstance)))) 1.0))))

(event Custom|OnGameStartEvent_Event
  (bind _foundwidgets (Widget|GetAllWidgetsOfClass "/Game/dylan/W_HUD.W_HUD_C" true))
  (EventDispatchers|AssignOnMinigameTimerEnd (Utilities|Array|Get(acopy) _foundwidgets) (delegate Custom|OnMinigameTimerEnd_Event)))

(event EventStartInteracting
  (params (Instigator :type Actor%20Object%20Reference))
  (bind _text (Variables|Default|Gettext))
  (bind _eat_timer (Variables|Default|Geteat%20timer))
  (if (Variables|Default|GetCanEat)
    (Utilities|Time|SetTimerbyEvent (delegate Custom|EatFood) (Variables|Default|GetInteractDelay))
    (Development|PrintString "started eated")
    (Variables|Default|SetIsBeingEaten true)
    (if (not (Variables|/Script/Engine.SceneComponent|GetbVisible _eat_timer))
      (Rendering|SetVisibility _eat_timer true false)
      (if (Variables|/Script/Engine.SceneComponent|GetbVisible _text)
        (Rendering|SetVisibility _text false false)))))

(event EventBeginPlay
  (Utilities|FlowControl|Sequence
    (:then_0
      ;[0 0 0 0.5] Get Camera reference
      (bind _returnvalue (Actor|GetActorOfClass "/Game/Paw_ism/Core/Camera/BP_GamePlayCamera.BP_GamePlayCamera_C"))
      (Variables|Default|SetCamera _returnvalue)
      (Rendering|SetVisibility (Variables|Default|Gettext) false false)
      (Rendering|SetVisibility (Variables|Default|Geteat%20timer) false false)
      (EventDispatchers|BindEventtoOnMouseEatenEvent (.AsBP%20My%20Game%20Instanc (Utilities|Casting|CastToBP_MyGameInstanc (Game|GetGameInstance))) (delegate Custom|ToggleEating))
      (bind _returnvalue_2 (Actor|GetActorOfClass "/Game/dylan/Minigame/BP_Spawner.BP_Spawner_C"))
      (Variables|Default|SetSpawner _returnvalue_2))
    (:then_1
      (EventDispatchers|AssignOnMouseEatenEvent (.AsBP%20My%20Game%20Instanc (Utilities|Casting|CastToBP_MyGameInstanc (Game|GetGameInstance))) (delegate Custom|OnMouseEatenEvent_Event)))
    (:then_2
      (Utilities|FlowControl|DelayUntilNextTick)
      (bind _foundwidgets (Widget|GetAllWidgetsOfClass "/Game/Paw_ism/Core/Widgets/W_StartMenu.W_StartMenu_C" true))
      (EventDispatchers|AssignOnGameStartEvent (Utilities|Array|Get(acopy) _foundwidgets) (delegate Custom|OnGameStartEvent_Event)))))

(event EventTick
  (params (DeltaSeconds :type Float%20%28single-precision%29))
  (bind _text (Variables|Default|Gettext))
  (bind _eat_timer (Variables|Default|Geteat%20timer))
  (Utilities|FlowControl|Sequence
    (:then_0
      (if (Variables|/Script/Engine.SceneComponent|GetbVisible _text)
        (Transformation|SetWorldRotation _text (Math|Rotator|FindLookatRotation (Transformation|GetWorldLocation _text) (Camera|GetCameraLocation (Game|GetPlayerCameraManager 0))) false false)))
    (:then_1
      (if (Variables|Default|GetIsBeingEaten)
        (Transformation|SetWorldRotation _eat_timer (Math|Rotator|FindLookatRotation (Transformation|GetWorldLocation _eat_timer) (Camera|GetCameraLocation (Game|GetPlayerCameraManager 0))) false false)
        (Default|SetPercent (.AsW%20Food%20Eating%20Timer (Utilities|Casting|CastToW_FoodEatingTimer (UserInterface|GetWidget (Variables|Default|Geteat%20timer)))) (/ (Class|KismetSystemLibrary|GetTimerElapsedTime 0 "EatFood") (Variables|Default|GetInteractDelay)))))))

(event EventStopInteracting
  (params (Instigator :type Actor%20Object%20Reference))
  (bind _eat_timer (Variables|Default|Geteat%20timer))
  (bind _text (Variables|Default|Gettext))
  (Utilities|Time|ClearTimerbyFunctionName 0 "EatFood")
  (Development|PrintString "stopped eating")
  (Variables|Default|SetIsBeingEaten false)
  (if (Variables|/Script/Engine.SceneComponent|GetbVisible _eat_timer)
    (Rendering|SetVisibility _eat_timer false false)
    (if (not (Variables|/Script/Engine.SceneComponent|GetbVisible _text))
      (Rendering|SetVisibility _text true false))))

(fn ConstructionScript)