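; Interactable pentagram that can be drawn once the game instance reports all mice are eaten.
; Interacting starts a draw timer and a praying montage on BP_ThirdPersonCharacter; either completing swaps the plane's material and notifies the game instance.
; A BP_Cat overlap shows a camera-facing info bubble; leaving hides it and clears the timer.
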(event OnComponentBeginOverlap(Plane)
  (params (OverlappedComponent :type Primitive%20Component%20Object%20Reference) (OtherActor :type Actor%20Object%20Reference) (OtherComp :type Primitive%20Component%20Object%20Reference) (OtherBodyIndex :type Integer) (bFromSweep :type Boolean) (SweepResult :type Hit%20Result%20Structure%20%28by%20ref%29))
  (bind _infobubble (Variables|Default|GetInfoBubble))
  (Utilities|Casting|CastToBP_Cat OtherActor)
  (if (not (Variables|/Script/Engine.SceneComponent|GetbVisible _infobubble))
    (Rendering|SetVisibility _infobubble true false)))

(event OnComponentEndOverlap(Plane)
  (params (OverlappedComponent :type Primitive%20Component%20Object%20Reference) (OtherActor :type Actor%20Object%20Reference) (OtherComp :type Primitive%20Component%20Object%20Reference) (OtherBodyIndex :type Integer))
  (bind _infobubble (Variables|Default|GetInfoBubble))
  (Utilities|Casting|CastToBP_Cat OtherActor)
  (Utilities|FlowControl|Sequence
    (:then_0
      (CallFunction|StopInteracting (Variables|Default|GetInstigator_1)))
    (:then_1
      (Utilities|FlowControl|DelayUntilNextTick)
      (if (Variables|/Script/Engine.SceneComponent|GetbVisible _infobubble)
        (Rendering|SetVisibility _infobubble false false)))))

(event Custom|OnMouseEatenEvent_Event
  (Variables|Default|SetCanDrawPentagran (== (Default|GetTotalMicePercent (.AsBP%20My%20Game%20Instanc (Utilities|Casting|CastToBP_MyGameInstanc (Game|GetGameInstance)))) 1.0)))

(event Custom|DrawPentagram
  (Rendering|Material|SetMaterial (Variables|Default|GetPlane) 0 "/Game/dylan/M_PENTAGRAMRAAAAAAAAAAAAAAAAAHHHHH.M_PENTAGRAMRAAAAAAAAAAAAAAAAAHHHHH")
  (Variables|Default|SetIsPentagramDrawn true)
  (Default|PentagramDrawn (.AsBP%20My%20Game%20Instanc (Utilities|Casting|CastToBP_MyGameInstanc (Game|GetGameInstance)))))

(event EventStartInteracting
  (params (Instigator :type Actor%20Object%20Reference))
  (if (not (Variables|Default|GetIsPentagramDrawn))
    (if (Variables|Default|GetCanDrawPentagran)
      (Utilities|Time|SetTimerbyEvent (delegate Custom|DrawPentagram) (Variables|Default|GetPentagranDrawingTime))
      (bind _output_get (Variables|Default|SetInstigator_1 Instigator))
      (bind _asbp_third_person_character (Utilities|Casting|CastToBP_ThirdPersonCharacter _output_get))
      (Animation|Montage|PlayMontage (Variables|/Script/Engine.Character|GetMesh _asbp_third_person_character) "/Game/dylan/animations/Praying_Anim1_Montage.Praying_Anim1_Montage" 2.0 0.0 "None" false
        (:OnCompleted
          (Rendering|Material|SetMaterial (Variables|Default|GetPlane) 0 "/Game/dylan/M_PENTAGRAMRAAAAAAAAAAAAAAAAAHHHHH.M_PENTAGRAMRAAAAAAAAAAAAAAAAAHHHHH")
          (Variables|Default|SetIsPentagramDrawn true)
          (Default|PentagramDrawn (.AsBP%20My%20Game%20Instanc (Utilities|Casting|CastToBP_MyGameInstanc (Game|GetGameInstance)))))))))

(event EventBeginPlay
  (EventDispatchers|AssignOnMouseEatenEvent (.AsBP%20My%20Game%20Instanc (Utilities|Casting|CastToBP_MyGameInstanc (Game|GetGameInstance))) (delegate Custom|OnMouseEatenEvent_Event))
  (Rendering|SetVisibility (Variables|Default|GetInfoBubble) false false))

(event EventStopInteracting
  (params (Instigator :type Actor%20Object%20Reference))
  (Utilities|Time|ClearTimerbyFunctionName 0 "DrawPentagram"))

(event EventTick
  (params (DeltaSeconds :type Float%20%28single-precision%29))
  (bind _infobubble (Variables|Default|GetInfoBubble))
  (if (Variables|/Script/Engine.SceneComponent|GetbVisible _infobubble)
    (Transformation|SetWorldRotation _infobubble (Math|Rotator|FindLookatRotation (Transformation|GetWorldLocation _infobubble) (Camera|GetCameraLocation (Game|GetPlayerCameraManager 0))) false false)))

(fn ConstructionScript)