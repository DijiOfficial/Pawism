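; Blood line actor that fades into view with a blood effect when the cat crosses it after it has been activated.
; BeginPlay toggles the line's visibility, and Activate arms the overlap trigger.
; An overlap by BP_Cat disarms it, toggles visibility again and runs a timeline driving FadeAmount on a dynamic M_FadeIn material.
; A DoOnce on the timeline update spawns the Niagara blood effect at EffectLocation.
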(event EventBeginPlay
  (Rendering|ToggleVisibility (Variables|Default|GetBloodLine) false))

(event Collision|EventActorBeginOverlap
  (params (OtherActor :type Actor%20Object%20Reference))
  ;[0 0 0 0.5] Triangle Is Active?
  (if (Variables|Default|GetbActive)
    (Utilities|Casting|CastToBP_Cat OtherActor)
    (Variables|Default|SetbActive false)
    (Rendering|ToggleVisibility (Variables|Default|GetBloodLine) false)
    (bind _returnvalue (Rendering|Material|CreateDynamicMaterialInstance "/Game/adam/Materials/M_FadeIn.M_FadeIn" "None" "None" :!class /Script/Engine.KismetMaterialLibrary))
    (Variables|Default|SetBloodLineMaterial _returnvalue)
    (Rendering|Material|SetMaterial (Variables|Default|GetBloodLine) 0 (Variables|Default|GetBloodLineMaterial))
    (bind _time (Timeline|Timeline Play)
      (:Update
        (Rendering|Material|SetScalarParameterValue (Variables|Default|GetBloodLineMaterial) "FadeAmount" _time :!class /Script/Engine.MaterialInstanceDynamic)
        (Utilities|FlowControl|DoOnce false
          (:Completed
            (Niagara|SpawnSystematLocation "/Game/adam/FX/NS_Blood.NS_Blood" (Transformation|GetWorldLocation (Variables|Default|GetEffectLocation)))))))))

(fn ConstructionScript)

(fn Activate
  (Variables|Default|SetbActive true))