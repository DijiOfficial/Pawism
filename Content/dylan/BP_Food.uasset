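; BP_Food is a food actor that shows a text label when the player character is near it.
; The text starts hidden and toggles on and off as BP_ThirdPersonCharacter enters and leaves the PickeableCollision volume.
; While visible, the text rotates every Tick to face the player camera.
; The graph holds no pickup or consumption logic, only this proximity prompt.
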(event OnComponentBeginOverlap(PickeableCollision)
  (params (OverlappedComponent :type Primitive%20Component%20Object%20Reference) (OtherActor :type Actor%20Object%20Reference) (OtherComp :type Primitive%20Component%20Object%20Reference) (OtherBodyIndex :type Integer) (bFromSweep :type Boolean) (SweepResult :type Hit%20Result%20Structure%20%28by%20ref%29))
  (bind _text (Variables|Default|Gettext))
  (Utilities|Casting|CastToBP_ThirdPersonCharacter OtherActor)
  (if (not (Variables|/Script/Engine.SceneComponent|GetbVisible _text))
    (Rendering|SetVisibility _text true false)))

(event OnComponentEndOverlap(PickeableCollision)
  (params (OverlappedComponent :type Primitive%20Component%20Object%20Reference) (OtherActor :type Actor%20Object%20Reference) (OtherComp :type Primitive%20Component%20Object%20Reference) (OtherBodyIndex :type Integer))
  (bind _text (Variables|Default|Gettext))
  (Utilities|Casting|CastToBP_ThirdPersonCharacter OtherActor)
  (if (Variables|/Script/Engine.SceneComponent|GetbVisible _text)
    (Rendering|SetVisibility _text false false)))

(event EventBeginPlay
  (Rendering|SetVisibility (Variables|Default|Gettext) false false))

(event EventTick
  (params (DeltaSeconds :type Float%20%28single-precision%29))
  (bind _text (Variables|Default|Gettext))
  (if (Variables|/Script/Engine.SceneComponent|GetbVisible _text)
    (Transformation|SetWorldRotation _text (Math|Rotator|FindLookatRotation (Transformation|GetWorldLocation _text) (Camera|GetCameraLocation (Game|GetPlayerCameraManager 0))) false false)))

(fn ConstructionScript)