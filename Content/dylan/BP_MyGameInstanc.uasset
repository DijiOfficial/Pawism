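; Game instance Blueprint that tracks level progress through mice eaten and pentagrams drawn.
; AddMouse increments the mouse count and fires the mouse-eaten event, while GetTotalMicePercent returns that count as a fraction of MiceNeeded.
; PentagramDrawn counts pentagrams, announces level end through the all-pentagrams-drawn event at five, and resets the mouse count, firing the mouse-eaten event again.
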(fn GetTotalMicePercent
  (return (/ (Math|Conversions|ToFloat(Integer) (Variables|Default|GetTotalMiceEaten)) (Variables|Default|GetMiceNeeded))))

(fn AddMouse
  (Math|Integer|IncrementInt (Variables|Default|GetTotalMiceEaten)
    (:%20%20
      (Default|CallOnMouseEatenEvent))))

(fn PentagramDrawn
  (bind _result (Math|Integer|IncrementInt (Variables|Default|GetTotalPentagramsDrawn))
    (:%20%20
      (if (>= _result 5)
        (Development|PrintString "Level Ended")
        (Default|CallOnAllPentagramsDrawnEvent))
      (Variables|Default|SetTotalMiceEaten 0)
      (Default|CallOnMouseEatenEvent))))